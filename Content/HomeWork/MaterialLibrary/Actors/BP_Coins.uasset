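; BP_Coins is a coin bag pickup that BP_ThirdPersonCharacter collects by interaction.
; Overlap toggles its TextCoin label and sets or clears the character's LookingAtActor, while Tick turns the label toward the camera by yaw only.
; Interact locks walking and flags Pickup, then uses timed delays to set Coin to Money, hide the bag, release the player and destroy itself.
; SendQuantities is an empty stub.
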(event `self.ReceiveBeginPlay`
  ;[1 0 0] Var Player Char
  (bind _asthird_person_character (cast `/Game/IMLearning/Characters/MainCharacter/BP_ThirdPersonCharacter` (`GameplayStatics.GetPlayerCharacter` 0)))
  (set `self.Player_Char` _asthird_person_character))

(event `self.ReceiveActorBeginOverlap`
  (params (OtherActor :type "Actor Object Reference"))
  ;[1 0.9479 0.9799] Comment Visibility
  (`SceneComponent.SetVisibility` (`self.Text_Coin`) true false)
  (set `/Game/IMLearning/Characters/MainCharacter/BP_ThirdPersonCharacter.LookingAtActor` self (`self.Player_Char`)))

(event `self.ReceiveActorEndOverlap`
  (params (OtherActor :type "Actor Object Reference"))
  ;[1 0.9479 0.9799] Comment Visibility
  (`SceneComponent.SetVisibility` (`self.Text_Coin`) false false)
  (set `/Game/IMLearning/Characters/MainCharacter/BP_ThirdPersonCharacter.LookingAtActor` null (`self.Player_Char`)))

(event `self.ReceiveTick`
  (params (DeltaSeconds :type "Float (single-precision)"))
  (bind _text_coin (`self.Text_Coin`))
  ;[1 0.7196 0] Rotate Text
  (`SceneComponent.K2_SetWorldRotation` _text_coin (`KismetMathLibrary.MakeRotator` 0.0 0.0 (.yaw (.rotation (`self.GetTransform` (`GameplayStatics.GetPlayerCameraManager` 0))))) false false)
  (`SceneComponent.K2_AddWorldRotation` _text_coin (struct :`Yaw` -180.0) false false))

(event `/Game/HomeWork/MaterialLibrary/BPI_Interface.Interact`
  (params (Money :type "Float (single-precision)") (BpRef :type "Object Object Reference"))
  (bind _player_char (`self.Player_Char`))
  (bind _player_char_2 (`self.Player_Char`))
  ;[1 0.3144 0] Collect Coin
  (set `/Game/IMLearning/Characters/MainCharacter/BP_ThirdPersonCharacter.Pickup` true _player_char_2)
  (set `/Game/IMLearning/Characters/MainCharacter/BP_ThirdPersonCharacter.CanWalk` false _player_char_2)
  (`KismetSystemLibrary.Delay` 1.0)
  (set `/Game/IMLearning/Characters/MainCharacter/BP_ThirdPersonCharacter.Coin` Money (`self.Player_Char`))
  (`SceneComponent.SetVisibility` (`self.Bag`) false true)
  (`KismetSystemLibrary.Delay` 0.73)
  (set `/Game/IMLearning/Characters/MainCharacter/BP_ThirdPersonCharacter.Pickup` false _player_char)
  (set `/Game/IMLearning/Characters/MainCharacter/BP_ThirdPersonCharacter.CanWalk` true _player_char)
  (`self.K2_DestroyActor`))

(fn `Send_Quantities`
  (params (Cube :type Integer) (Cylinder :type Integer) (Pyramid :type Integer))
  (return))

(fn `UserConstructionScript`)