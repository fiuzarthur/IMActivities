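; Playable pinball machine that the third-person character interacts with to toggle a blended camera view and lock walking.
; Tick polls the character's input flags, driving timelines for flippers, table tilt and plunger, each stage chained from the previous timeline's Update.
; With no ball present, it spawns blue and pink balls alternately.
; The drain box or exiting destroys the ball and opens the wedge gate, which blocks again after an overlap ends.
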(event `self.ReceiveTick`
  (params (DeltaSeconds :type "Float (single-precision)"))
  (bind _returnvalue (`KismetMathLibrary.Conv_RotatorToVector` (`self.GameRotation`)))
  (bind _returnvalue_2 (`SceneComponent.K2_GetComponentLocation` (`self.Spawn_box`)))
  ;[1 0 0] Tick
  ;;[0 1 0.9783] Movimento Paleta Esquerda
  (if (`/Game/IMLearning/Characters/MainCharacter/BP_ThirdPersonCharacter.L_Pin` (`self.Player_Char`))
    (bind (_direction _track1) (`Timeline|TimelineLRot` :!label _label)
      (:`Update`
        (`SceneComponent.K2_SetRelativeRotation` (`self.Flipper_L`) (`KismetMathLibrary.RLerp` (`self.Flipper_LRotMin`) (`self.Flipper_LRotMax`) _track1) false false)
        ;;[1 0.11 0.9618] Movimento Paleta Direita
        (if (`/Game/IMLearning/Characters/MainCharacter/BP_ThirdPersonCharacter.R_Pin` (`self.Player_Char`))
          (bind (_direction_2 _track1_2) (`Timeline|TimelineRRot` :!label _label_2)
            (:`Update`
              (`SceneComponent.K2_SetRelativeRotation` (`self.Flipper_R`) (`KismetMathLibrary.RLerp` (`self.Flipper_RRotMin`) (struct :`Pitch` -40.0 :`Roll` -90.0) _track1_2) false false)
              ;;[1 0.4095 0] Tilt
              (if (`/Game/IMLearning/Characters/MainCharacter/BP_ThirdPersonCharacter.Tilting` (`self.Player_Char`))
                (bind (_direction_3 _track1_3) (`Timeline|Timeline_0` :!via `PlayFromStart`)
                  (:`Update`
                    (`SceneComponent.K2_SetRelativeRotation` (`self.Game`) (`KismetMathLibrary.RLerp` (`KismetMathLibrary.Conv_VectorToRotator` (+ _returnvalue (0.0 0.0 -0.2))) (`KismetMathLibrary.Conv_VectorToRotator` (+ _returnvalue (0.0 0.0 0.2))) _track1_3) false false))))
              (if (`self.BallExists`)
                ;;[0.6499 0.02034 1] Lançador da bola(G)
                (if (`/Game/IMLearning/Characters/MainCharacter/BP_ThirdPersonCharacter.Throw` (`self.Player_Char`))
                  (bind (_direction_4 _newtrack_0) (`Timeline|Timeline_01` :!label _label_3)
                    (:`Update`
                      (set `self.TrackLaunch` _newtrack_0)
                      (if (`self.IsLaunch`)
                        (set `self.TrackLaunch` (`KismetMathLibrary.FClamp` (* (`self.TrackLaunch`) 0.82))))
                      (`SceneComponent.K2_SetRelativeLocation` (`self.Impulse`) (`KismetMathLibrary.VLerp` (43.0 211.19313 -28.0) (43.0 211.19313 -44.0) (`self.TrackLaunch`)) false false))
                    (:`Finished`
                      (set `self.IsLaunch` false)))
                  (else
                    (set `self.IsLaunch` true)
                    (goto _label_3 :!via `Reverse`)))
                (else
                  ;;[0.009985 0 1] Spawn das bolas alternadamente
                  (`/Engine/EditorBlueprintResources/StandardMacros.FlipFlop`
                    (:`A`
                      (bind _returnvalue_3 (`|SpawnActorFromClass` "/Game/HomeWork/MaterialLibrary/Actors/BPC_BlueBall.BPC_BlueBall_C" (`KismetMathLibrary.MakeTransform` _returnvalue_2 (struct) (0.13 0.13 0.13)) "Undefined" "OverrideRootScale" null null))
                      (set `self.Ball` _returnvalue_3))
                    (:`B`
                      (bind _returnvalue_4 (`|SpawnActorFromClass` "/Game/HomeWork/MaterialLibrary/Actors/BP_PinkBall.BP_PinkBall_C" (`KismetMathLibrary.MakeTransform` _returnvalue_2 (struct) (0.13 0.13 0.13)) "Undefined" "OverrideRootScale" null null))
                      (set `self.Ball` _returnvalue_4)))
                  (set `self.BallExists` true)))))
          (else
            (goto _label_2 :!via `Reverse`)))))
    (else
      (goto _label :!via `Reverse`))))

(event `self.ReceiveBeginPlay`
  ;[1 0.3126 0] Set Var
  (set `self.Flipper_LRotMin` (`SceneComponent.RelativeRotation` (`self.Flipper_L`)))
  (set `self.Flipper_RRotMin` (`SceneComponent.RelativeRotation` (`self.Flipper_R`)))
  (bind _asthird_person_character (cast `/Game/IMLearning/Characters/MainCharacter/BP_ThirdPersonCharacter` (`GameplayStatics.GetPlayerCharacter` 0)))
  (set `self.Player_Char` _asthird_person_character)
  (set `self.GameRotation` (`SceneComponent.RelativeRotation` (`self.Game`))))

(event `/Game/HomeWork/MaterialLibrary/BPI_Interface.Interact`
  (params (Money :type "Float (single-precision)") (BpRef :type "Object Object Reference"))
  (bind _returnvalue (`GameplayStatics.GetPlayerController` 0))
  (bind _player_char (`self.Player_Char`))
  (bind _player_char_2 (`self.Player_Char`))
  ;[0 0 0] Set Camera ToPinball
  (`/Engine/EditorBlueprintResources/StandardMacros.FlipFlop`
    (:`A`
      (`PlayerController.SetViewTargetWithBlend` _returnvalue self 2.0 "VTBlend_Linear" 0.0 false)
      (set `/Game/IMLearning/Characters/MainCharacter/BP_ThirdPersonCharacter.Is_Interactig` true _player_char)
      (set `/Game/IMLearning/Characters/MainCharacter/BP_ThirdPersonCharacter.CanWalk` false _player_char_2))
    (:`B`
      (`PlayerController.SetViewTargetWithBlend` _returnvalue (`self.Player_Char`) 0.0 "VTBlend_Linear" 0.0 false)
      (set `/Game/IMLearning/Characters/MainCharacter/BP_ThirdPersonCharacter.Is_Interactig` false _player_char)
      (set `/Game/IMLearning/Characters/MainCharacter/BP_ThirdPersonCharacter.CanWalk` true _player_char_2)
      (`self.K2_DestroyActor` (`self.Ball`))
      (set `self.BallExists` false)
      (`PrimitiveComponent.SetCollisionProfileName` (`self.WedgeExit`) "OverlapAll" true))))

(event `self.DestroyBox.OnComponentBeginOverlap`
  (params (OverlappedComponent :type "PrimitiveComponent Object Reference") (OtherActor :type "Actor Object Reference") (OtherComp :type "PrimitiveComponent Object Reference") (OtherBodyIndex :type Integer) (bFromSweep :type Boolean) (SweepResult :type "HitResult Structure (by ref)"))
  ;[0 0.8094 1] Destroy Ball and set to respawn
  (`self.K2_DestroyActor` OtherActor)
  (set `self.BallExists` false)
  (`PrimitiveComponent.SetCollisionProfileName` (`self.WedgeExit`) "OverlapAll" true))

(event `self.ColBox.OnComponentBeginOverlap`
  (params (OverlappedComponent :type "PrimitiveComponent Object Reference") (OtherActor :type "Actor Object Reference") (OtherComp :type "PrimitiveComponent Object Reference") (OtherBodyIndex :type Integer) (bFromSweep :type Boolean) (SweepResult :type "HitResult Structure (by ref)"))
  (bind _asthird_person_character (cast `/Game/IMLearning/Characters/MainCharacter/BP_ThirdPersonCharacter` OtherActor))
  (set `/Game/IMLearning/Characters/MainCharacter/BP_ThirdPersonCharacter.LookingAtActor` self _asthird_person_character))

(event `self.WedgeExit.OnComponentEndOverlap`
  (params (OverlappedComponent :type "PrimitiveComponent Object Reference") (OtherActor :type "Actor Object Reference") (OtherComp :type "PrimitiveComponent Object Reference") (OtherBodyIndex :type Integer))
  ;[0 0.9931 1] Close The Gate
  (`PrimitiveComponent.SetCollisionProfileName` (`self.WedgeExit`) "BlockAll" true))

(event `self.ColBox.OnComponentEndOverlap`
  (params (OverlappedComponent :type "PrimitiveComponent Object Reference") (OtherActor :type "Actor Object Reference") (OtherComp :type "PrimitiveComponent Object Reference") (OtherBodyIndex :type Integer))
  (bind _asthird_person_character (cast `/Game/IMLearning/Characters/MainCharacter/BP_ThirdPersonCharacter` OtherActor))
  (set `/Game/IMLearning/Characters/MainCharacter/BP_ThirdPersonCharacter.LookingAtActor` null _asthird_person_character))

(fn `UserConstructionScript`)