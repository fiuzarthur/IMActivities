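; BP_Elevator is an elevator actor that moves its mesh vertically when activated.
; Each Activate call alternates through a FlipFlop between playing and reversing the Elevator timeline.
; On update, the timeline's T1 track, scaled by Height, sets the mesh's relative Z location without sweep.
; BeginPlay sets the timeline play rate to the inverse of Time, so that variable controls travel duration.
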(event `self.ReceiveBeginPlay`
  (`TimelineComponent.SetPlayRate` (`self.Elevator`) (/ 1.0 (`self.Time`))))

(event `/Game/HomeWork/Library/BPI_Actions.Activate`
  (`/Engine/EditorBlueprintResources/StandardMacros.FlipFlop`
    (:`A`
      (bind (_direction _t1) (`Timeline|Elevator` :!label _label)
        (:`Update`
          (`SceneComponent.K2_SetRelativeLocation` (`self.ElevatorMesh`) (`KismetMathLibrary.MakeVector` 0.0 0.0 (* _t1 (`self.Height`))) false false))))
    (:`B`
      (goto _label :!via `Reverse`))))

(fn `UserConstructionScript`)