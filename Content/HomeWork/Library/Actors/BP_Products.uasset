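; BP_Products is a collectible world item whose mesh follows its StructItem category: pyramid, cylinder, cube, or heal/mana potion.
; Overlap shows a camera-yaw-facing text label and registers the item as the player's LookingAtActor.
; Interact briefly locks walking, hides the mesh, then checks collectability, slot count and carry weight.
; Success updates weight, inventory widget and shape counters, then destroys the actor; failed checks leave it invisible.
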(event `/Game/HomeWork/Library/BP_Interface.Interact`
  (params (Money :type "Float (single-precision)") (BpRef :type "Object Object Reference"))
  (bind _player_char (`self.Player_Char`))
  (bind _struct_item (`self.Struct_Item`))
  (bind _player_char_2 (`self.Player_Char`))
  (bind _player_char_3 (`self.Player_Char`))
  (bind _player_char_4 (`self.Player_Char`))
  (bind _player_char_5 (`self.Player_Char`))
  (bind _player_char_6 (`self.Player_Char`))
  (bind _player_char_7 (`self.Player_Char`))
  (bind ((`Weight_12_102B73F941EC008EEAC2168C20B2FDC6` _weight) (`Quantity_15_3552B3194DDCCEBE2AAF56B2B4CE9A93` _quantity)) (break `/Game/HomeWork/Library/Struct_Itens` (`self.Struct_Item`)))
  (bind ((`Quantity_15_3552B3194DDCCEBE2AAF56B2B4CE9A93` _quantity_2)) (break `/Game/HomeWork/Library/Struct_Itens` (`self.Struct_Item`)))
  (bind _returnvalue (+ (* _quantity _weight) (`/Game/IMLearning/Characters/MainCharacter/ThirdPersonCharacter.Weight` _player_char_2)))
  ;[1 1 1] On overlap collect item
  (set `/Game/IMLearning/Characters/MainCharacter/ThirdPersonCharacter.Pickup` true _player_char_3)
  (set `/Game/IMLearning/Characters/MainCharacter/ThirdPersonCharacter.CanWalk` false _player_char_3)
  (`KismetSystemLibrary.Delay` 1.0)
  (`SceneComponent.SetVisibility` (`self.Item_Mesh`) false true)
  (`KismetSystemLibrary.Delay` 0.75)
  (set `/Game/IMLearning/Characters/MainCharacter/ThirdPersonCharacter.Pickup` false _player_char)
  (set `/Game/IMLearning/Characters/MainCharacter/ThirdPersonCharacter.CanWalk` true _player_char)
  (if (`.Collectable_22_0B1DB350457A5397B45B8CA767CC30B8` (break `/Game/HomeWork/Library/Struct_Itens` (`self.Struct_Item`)))
    (if (< (`/Game/IMLearning/Characters/MainCharacter/ThirdPersonCharacter.Inventory_Quant` (`self.Player_Char`)) 5)
      (if (<= _returnvalue (`/Game/IMLearning/Characters/MainCharacter/ThirdPersonCharacter.WeightMAX` _player_char_2))
        (set `/Game/IMLearning/Characters/MainCharacter/ThirdPersonCharacter.Weight` _returnvalue _player_char_4)
        (`/Game/HomeWork/Library/WBP_Status.Item_To_Inventory_Event` (`/Game/IMLearning/Characters/MainCharacter/ThirdPersonCharacter.Widget` _player_char_4) _struct_item)
        (switch `/Game/HomeWork/Library/Enum_Category` (`.Category_9_F58949BD46723E4CBA5A3F83A0F8CFFC` (break `/Game/HomeWork/Library/Struct_Itens` _struct_item))
          (:`NewEnumerator2`
            (set `/Game/IMLearning/Characters/MainCharacter/ThirdPersonCharacter.PyramidQuanti` (+ (`/Game/IMLearning/Characters/MainCharacter/ThirdPersonCharacter.PyramidQuanti` _player_char_6) _quantity_2) _player_char_6))
          (:`NewEnumerator1`
            (set `/Game/IMLearning/Characters/MainCharacter/ThirdPersonCharacter.CylinderQuanti` (+ _quantity_2 (`/Game/IMLearning/Characters/MainCharacter/ThirdPersonCharacter.CylinderQuanti` _player_char_7)) _player_char_7))
          (:`NewEnumerator0`
            (set `/Game/IMLearning/Characters/MainCharacter/ThirdPersonCharacter.CubeQuanti` (+ _quantity_2 (`/Game/IMLearning/Characters/MainCharacter/ThirdPersonCharacter.CubeQuanti` _player_char_5)) _player_char_5))
          (:`NewEnumerator3`
            _)
          (:`NewEnumerator4`
            _))
        (`self.K2_DestroyActor`)))))

(event `self.ReceiveBeginPlay`
  ;[1 1 1] Set Static Mesh
  (bind _asthird_person_character (cast `/Game/IMLearning/Characters/MainCharacter/ThirdPersonCharacter` (`GameplayStatics.GetPlayerCharacter` 0)))
  (set `self.Player_Char` _asthird_person_character)
  (switch `/Game/HomeWork/Library/Enum_Category` (`.Category_9_F58949BD46723E4CBA5A3F83A0F8CFFC` (break `/Game/HomeWork/Library/Struct_Itens` (`self.Struct_Item`)))
    (:`NewEnumerator2`
      (`StaticMeshComponent.SetStaticMesh` (`self.Item_Mesh`) "/Game/IMLearning/Geometries/Shape_QuadPyramid.Shape_QuadPyramid"))
    (:`NewEnumerator1`
      (`StaticMeshComponent.SetStaticMesh` (`self.Item_Mesh`) "/Game/IMLearning/Geometries/Shape_Cylinder.Shape_Cylinder"))
    (:`NewEnumerator0`
      (`StaticMeshComponent.SetStaticMesh` (`self.Item_Mesh`) "/Game/IMLearning/Geometries/1M_Cube.1M_Cube"))
    (:`NewEnumerator3`
      (`StaticMeshComponent.SetStaticMesh` (`self.Item_Mesh`) "/Game/HomeWork/Library/Mesh/PotionHeal.PotionHeal"))
    (:`NewEnumerator4`
      (`StaticMeshComponent.SetStaticMesh` (`self.Item_Mesh`) "/Game/HomeWork/Library/Mesh/PotioN_Mana.PotioN_Mana"))))

(event `self.ReceiveTick`
  (params (DeltaSeconds :type "Float (single-precision)"))
  (bind _textrender (`self.TextRender`))
  (`SceneComponent.K2_SetWorldRotation` _textrender (`KismetMathLibrary.MakeRotator` 0.0 0.0 (.yaw (.rotation (`self.GetTransform` (`GameplayStatics.GetPlayerCameraManager` 0))))) false false)
  (`SceneComponent.K2_AddWorldRotation` _textrender (struct :`Yaw` -180.0) false false))

(event `self.ReceiveActorBeginOverlap`
  (params (OtherActor :type "Actor Object Reference"))
  (cast `/Game/IMLearning/Characters/MainCharacter/ThirdPersonCharacter` OtherActor)
  (`SceneComponent.SetVisibility` (`self.TextRender`) true false)
  (set `/Game/IMLearning/Characters/MainCharacter/ThirdPersonCharacter.LookingAtActor` self (`self.Player_Char`)))

(event `self.ReceiveActorEndOverlap`
  (params (OtherActor :type "Actor Object Reference"))
  (cast `/Game/IMLearning/Characters/MainCharacter/ThirdPersonCharacter` OtherActor)
  (`SceneComponent.SetVisibility` (`self.TextRender`) false false)
  (set `/Game/IMLearning/Characters/MainCharacter/ThirdPersonCharacter.LookingAtActor` null (`self.Player_Char`)))

(fn `UserConstructionScript`
  (switch `/Game/HomeWork/Library/Enum_Category` (`.Category_9_F58949BD46723E4CBA5A3F83A0F8CFFC` (break `/Game/HomeWork/Library/Struct_Itens` (`self.Struct_Item`)))
    (:`NewEnumerator2`
      (`StaticMeshComponent.SetStaticMesh` (`self.Item_Mesh`) "/Game/IMLearning/Geometries/Shape_QuadPyramid.Shape_QuadPyramid"))
    (:`NewEnumerator1`
      (`StaticMeshComponent.SetStaticMesh` (`self.Item_Mesh`) "/Game/IMLearning/Geometries/Shape_Cylinder.Shape_Cylinder"))
    (:`NewEnumerator0`
      (`StaticMeshComponent.SetStaticMesh` (`self.Item_Mesh`) "/Game/IMLearning/Geometries/1M_Cube.1M_Cube"))
    (:`NewEnumerator3`
      (`StaticMeshComponent.SetStaticMesh` (`self.Item_Mesh`) "/Game/HomeWork/Library/Mesh/PotionHeal.PotionHeal"))
    (:`NewEnumerator4`
      (`StaticMeshComponent.SetStaticMesh` (`self.Item_Mesh`) "/Game/HomeWork/Library/Mesh/PotioN_Mana.PotioN_Mana"))))