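; BP_Store is a store actor for one item category (pyramid, cylinder or cube), labelled by text that turns with the player's camera.
; On Interact, if the player holds that category, it spawns a BP_Products at a scene component, then steps that component along, shifting rows halfway to capacity.
; It then removes the matching item from the player's inventory and widget.
; When full, it only prints "FECHADO".
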(event `self.ReceiveBeginPlay`
  ;[1 0 0] Begin Play
  ;;[1 0.7392 0.01289] Set Store Name
  (switch `/Game/HomeWork/Library/Enum_Category` (`.Category_9_F58949BD46723E4CBA5A3F83A0F8CFFC` (break `/Game/HomeWork/Library/Struct_Itens` (`self.Struct_Category`)))
    (:`NewEnumerator2`
      (set `self.Text` "Piramide"))
    (:`NewEnumerator1`
      (set `self.Text` "Cilindro"))
    (:`NewEnumerator0`
      (set `self.Text` "Cubo")))
  (`TextRenderComponent.K2_SetText` (`self.TextRender`) (`self.Text`))
  ;;[0 0.8505 1] Var Player
  (bind _asthird_person_character (cast `/Game/IMLearning/Characters/MainCharacter/ThirdPersonCharacter` (`GameplayStatics.GetPlayerCharacter` 0)))
  (set `self.Player_Char` _asthird_person_character))

(event `self.ReceiveTick`
  (params (DeltaSeconds :type "Float (single-precision)"))
  (bind _textrender (`self.TextRender`))
  ;[1 0 0] Rotate Text
  (`SceneComponent.K2_SetWorldRotation` _textrender (`KismetMathLibrary.MakeRotator` 0.0 0.0 (.yaw (.rotation (`self.GetTransform` (`GameplayStatics.GetPlayerCameraManager` 0))))) false false)
  (`SceneComponent.K2_AddWorldRotation` _textrender (struct :`Yaw` -180.0) false false))

(event `/Game/HomeWork/Library/BP_Interface.Interact`
  (params (Money :type "Float (single-precision)") (BpRef :type "Object Object Reference"))
  (bind _scenec (`self.SceneC`))
  (bind _player_char (`self.Player_Char`))
  (bind _scenec_2 (`self.SceneC`))
  (bind ((`Name_5_280C2B304A7C8AE31C7128B137258ED7` _name) (`Image_6_FB81B1E04D2A8C927989B0B275722AD8` _image) (`Category_9_F58949BD46723E4CBA5A3F83A0F8CFFC` _category) (`Quantity_15_3552B3194DDCCEBE2AAF56B2B4CE9A93` _quantity) (`Edable_18_1115CCE44A51DD2EB7799597FA7E1F15` _edable) (`Groupable_20_AA988EA446A45EB4478283B974EDFB1B` _groupable) (`Collectable_22_0B1DB350457A5397B45B8CA767CC30B8` _collectable)) (break `/Game/HomeWork/Library/Struct_Itens` (`self.Struct_Category`)))
  (bind (_relativelocation_x _relativelocation_y _relativelocation_z) (`KismetMathLibrary.BreakVector` (`SceneComponent.RelativeLocation` _scenec)))
  ;[1 0.4799 0] Interact
  (if (< (`self.ItemOnstore`) (`self.ItemMax`))
    ;;[1 0.8797 0] Switch Obj Category
    (switch `/Game/HomeWork/Library/Enum_Category` (`.Category_9_F58949BD46723E4CBA5A3F83A0F8CFFC` (break `/Game/HomeWork/Library/Struct_Itens` (`self.Struct_Category`)))
      (:`NewEnumerator2`
        (if (> (`/Game/IMLearning/Characters/MainCharacter/ThirdPersonCharacter.PyramidQuanti` _player_char) 0)
          ;;[0 0.574 1] Spawn Respective obj and move Scene component
          (`|SpawnActorFromClass` "/Game/HomeWork/Library/Actors/BP_Products.BP_Products_C" (`SceneComponent.K2_GetComponentToWorld` _scenec_2) "Undefined" "OverrideRootScale" null (`self.Struct_Category`) null :!label _label)
          (if (== (+ (`self.ItemOnstore`) 1) (/ (`self.ItemMax`) 2)) :!label _label_2
            (set `self.XMove` -20.0)
            (set `self.Ymove` 60.0))
          (`SceneComponent.K2_SetRelativeLocation` _scenec (`KismetMathLibrary.MakeVector` (+ _relativelocation_x (`self.XMove`)) (+ _relativelocation_y (`self.Ymove`)) _relativelocation_z) false false)
          (set `self.XMove` 0.0)
          (set `self.Ymove` -15.0)
          (`/Engine/EditorBlueprintResources/StandardMacros.IncrementInt` (`self.ItemOnstore`)
            (:`  `
              (bind (_item_found _has_item) (`/Game/HomeWork/Library/WBP_Status.Function_Find_Item` (`/Game/IMLearning/Characters/MainCharacter/ThirdPersonCharacter.Widget` (`self.Player_Char`)) (`self.Struct_Category`)))
              (if _has_item
                (bind _aswbp_generic_item (cast `/Game/HomeWork/Library/WBP_Generic_Item` _item_found))
                (bind _output_get (set `self.Struct_Category` (make `/Game/HomeWork/Library/Struct_Itens` _name _image _category (`.Weight_12_102B73F941EC008EEAC2168C20B2FDC6` (break `/Game/HomeWork/Library/Struct_Itens` (`/Game/HomeWork/Library/WBP_Generic_Item.Item_Category` _aswbp_generic_item))) _quantity _edable _groupable _collectable)))
                (`/Game/IMLearning/Characters/MainCharacter/ThirdPersonCharacter.Remove_Itens` (`self.Player_Char`) _output_get)
                (`/Game/HomeWork/Library/WBP_Generic_Item.Remove_Item` _aswbp_generic_item))))))
      (:`NewEnumerator1`
        (if (> (`/Game/IMLearning/Characters/MainCharacter/ThirdPersonCharacter.CylinderQuanti` _player_char) 0)
          (goto _label)))
      (:`NewEnumerator0`
        (if (> (`/Game/IMLearning/Characters/MainCharacter/ThirdPersonCharacter.CubeQuanti` _player_char) 0)
          (`|SpawnActorFromClass` "/Game/HomeWork/Library/Actors/BP_Products.BP_Products_C" (`KismetMathLibrary.MakeTransform` (`KismetMathLibrary.MakeVector` (.x (.location (`SceneComponent.K2_GetComponentToWorld` _scenec_2))) (.y (.location (`SceneComponent.K2_GetComponentToWorld` _scenec_2))) (+ (.z (.location (`SceneComponent.K2_GetComponentToWorld` _scenec_2))) 10.0)) (.rotation (`SceneComponent.K2_GetComponentToWorld` _scenec_2)) (.scale (`SceneComponent.K2_GetComponentToWorld` _scenec_2))) "Undefined" "OverrideRootScale" null (`self.Struct_Category`) null)
          (goto _label_2))))
    (else
      (`KismetSystemLibrary.PrintString` "FECHADO"))))

(fn `UserConstructionScript`)